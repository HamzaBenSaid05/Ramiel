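; BP_SoundTrack is the music manager that switches between tension, scattered, fight and death tracks as gameplay changes.
; At BeginPlay it starts tension music and binds to each AI character's see-player event, whose percent picks the track, and to the player's death, which overrides it.
; ChangeSoundTrack selects per-track fade durations, then runs timed fade-outs and fade-ins, using an IsChanging flag to ignore requests mid-transition except death.
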(event `self.ReceiveBeginPlay`
  (`self.ChangeSoundTrack` (`self.TensionSoundTrackSound`))
  (bind _outactors (`GameplayStatics.GetAllActorsOfClass` "/Script/GGJ_Mask.GGJ_AIBaseCharacter"))
  (bind _output_get (set `self.Enemies` _outactors))
  (for _array_element _output_get
    (add `GGJ_AIBaseCharacter.OnEnemySeePlayer` _array_element (delegate `CustomEvent`)))
  (bind _returnvalue (`GameplayStatics.GetActorOfClass` "/Game/Blueprint/Characters/Player/BP_Player.BP_Player_C"))
  (add `/Game/Blueprint/Characters/Player/BP_Player.OnDeath` _returnvalue (delegate `PlayerDeath`)))

(event `CustomEvent`
  (params (Percent :type "Float (single-precision)"))
  (if (`self.bPlayerDied`)
    _
    (elif (>= Percent 1.0)
      (`self.ChangeSoundTrack` (`self.FightSoundTrackAudio`))
      (elif (and (< Percent 1.0) (> Percent 0.0))
        (`self.ChangeSoundTrack` (`self.ScatteredSoundTrackAudio`))
        (else
          (`self.ChangeSoundTrack` (`self.TensionSoundTrackSound`)))))))

(event `PlayerDeath`
  (set `self.bPlayerDied` true)
  (set `self.bIsChanging` false)
  (`self.ChangeSoundTrack` (`self.DeathSoundTrackAudio`)))

(fn `ChangeSoundTrack`
  (params (CurrentSoundTrackAudio :type "SoundBase Object Reference"))
  ; Check if is not changinc sound
  (if (`self.bIsChanging`)
    (return)
    (else
      ; Check if is playing the same sound track
      (if (== (`local.CurrentSoundTrackAudio`) (`self.CurrentSoundTrackAudio`))
        (return)
        (else
          (`self.SetCutstomFadeInFadeOut` (`local.CurrentSoundTrackAudio`))
          ; if is not changing sound track, Set new sound track
          (set `self.CurrentSoundTrackAudio` (`local.CurrentSoundTrackAudio`))
          (if (`AudioComponent.IsPlaying` (`self.SoundTrack`))
            ; If is playing any sound, start fade out
            (`self.FadeOut` (`self.CurrentFadeOutDuration`))
            (else
              ; If is not playing any sound, change sound and start playing it
              (`self.SetSound`))))))))

(fn `FadeIn`
  (params (FadeInDuration :type "Float (single-precision)"))
  (`AudioComponent.FadeIn` (`self.SoundTrack`) FadeInDuration 1.0 0.0 "Linear")
  (`KismetSystemLibrary.PrintString` "Fade In")
  (`KismetSystemLibrary.K2_SetTimerDelegate` (`|CreateDelegate` :!event `PlaySound`) FadeInDuration))

(fn `FadeOut`
  (params (FadeOutDuration :type "Float (single-precision)"))
  (set `self.bIsChanging` true)
  (`AudioComponent.FadeOut` (`self.SoundTrack`) FadeOutDuration 0.0 "Linear")
  (`KismetSystemLibrary.PrintString` "Fade Out")
  (`KismetSystemLibrary.K2_SetTimerDelegate` (`|CreateDelegate` :!event `SetSound`) FadeOutDuration))

(fn `PlaySound`
  (set `self.bIsChanging` false))

(fn `ResetIsChanging`
  (params (NewSound :type "SoundBase Object Reference"))
  (`AudioComponent.SetSound` (`self.SoundTrack`) NewSound)
  (`AudioComponent.Play` (`self.SoundTrack`) 0.0))

(fn `SetCutstomFadeInFadeOut`
  (params (NewSound :type "SoundBase Object Reference"))
  (if (== NewSound (`self.ScatteredSoundTrackAudio`))
    (set `self.CurrentFadeInDuration` (`self.FadeInDurationScattered`))
    (set `self.CurrentFadeOutDuration` (`self.FadeOutDurationScattered`))
    (elif (== (`local.NewSound`) (`self.FightSoundTrackAudio`))
      (set `self.CurrentFadeInDuration` (`self.FadeInDurationFight`))
      (set `self.CurrentFadeOutDuration` (`self.FadeOutDurationFight`))
      (elif (== (`local.NewSound`) (`self.TensionSoundTrackSound`))
        (set `self.CurrentFadeInDuration` (`self.FadeInDurationTension`))
        (set `self.CurrentFadeOutDuration` (`self.FadeOutDurationTension`))
        (elif (== (`local.NewSound`) (`self.DeathSoundTrackAudio`))
          (set `self.CurrentFadeInDuration` (`self.FadeInDurationPlayerDeath`))
          (set `self.CurrentFadeOutDuration` (`self.FadeOutDurationPlayerDeath`)))))))

(fn `SetSound`
  (set `self.bIsChanging` true)
  (`AudioComponent.SetSound` (`self.SoundTrack`) (`self.CurrentSoundTrackAudio`))
  (`self.FadeIn` (`self.CurrentFadeInDuration`)))

(fn `UserConstructionScript`)