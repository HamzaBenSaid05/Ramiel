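; BP_KingDoor is the door that triggers the game's ending cinematic when the local player's character overlaps its box.
; The overlap hides the character and HUD, plays the assigned level sequence, then loads L_MainMenu as a level instance after a fixed delay.
; Sequence completion sets game over on GM_Mask.
; Functions swap in the open mesh, assign the sequence actor, and select ending A or B by whether the priest is possessed.
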(event `self.Box.OnComponentBeginOverlap`
  (params (OverlappedComponent :type "PrimitiveComponent Object Reference") (OtherActor :type "Actor Object Reference") (OtherComp :type "PrimitiveComponent Object Reference") (OtherBodyIndex :type Integer) (bFromSweep :type Boolean) (SweepResult :type "HitResult Structure (by ref)"))
  (bind _ascharacter (cast `Character` OtherActor))
  (if (== (`Pawn.GetController` _ascharacter) (`GameplayStatics.GetPlayerController` 0))
    (`self.SetActorHiddenInGame` (`GameplayStatics.GetPlayerCharacter` 0) true)
    (add `MovieSceneSequencePlayer.OnFinished` (`LevelSequenceActor.SequencePlayer` (`self.LevelSequenceActor`)) (delegate `OnFinished_Event`))
    (`Widget.SetVisibility` (`/Game/Blueprint/Characters/Player/PC_Player.HUD` (cast `/Game/Blueprint/Characters/Player/PC_Player` (`GameplayStatics.GetPlayerController` 0) :!pure true)) "Hidden")
    (`MovieSceneSequencePlayer.Play` (`LevelSequenceActor.SequencePlayer` (`self.LevelSequenceActor`)))
    (`KismetSystemLibrary.Delay` 12.0)
    (`LevelStreamingDynamic.LoadLevelInstanceBySoftObjectPtr` "/Game/LevelDesign/L_MainMenu.L_MainMenu" (0.0 0.0 0.0) (struct) "" null)))

(event `OnFinished_Event`
  (bind _asgm_mask (cast `/Game/Blueprint/GM_Mask` (`GameplayStatics.GetGameMode`)))
  (`/Game/Blueprint/GM_Mask.SetGameOver` _asgm_mask true))

(fn `ChangeLevelSequence`
  (params (bIsPriestPossesed :type Boolean))
  (if bIsPriestPossesed
    (bind _output_get (set `self.CurrentLevelSequence` "/Game/LevelSequence/LS_EndingB.LS_EndingB"))
    (`LevelSequenceActor.SetSequence` (`self.LevelSequenceActor`) _output_get)
    (else
      (bind _output_get_2 (set `self.CurrentLevelSequence` "/Game/LevelSequence/LS_EndingA.LS_EndingA"))
      (`LevelSequenceActor.SetSequence` (`self.LevelSequenceActor`) _output_get_2))))

(fn `OpenDoor`
  (`StaticMeshComponent.SetStaticMesh` (`self.StaticMesh`) (`self.DoorMeshOpen`)))

(fn `SetLevelSequenceActor`
  (params (LevelSequenceActor :type "LevelSequenceActor Object Reference"))
  (set `self.LevelSequenceActor` LevelSequenceActor))

(fn `UserConstructionScript`)