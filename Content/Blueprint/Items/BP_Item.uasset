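; BP_Item is an item actor that can be highlighted with an outline and is destroyed by any damage.
; The Overlay event toggles the MI_Outline overlay material on its static mesh together with the visibility of its widget, and BeginPlay switches both off.
; ReturnCurrentMesh exposes the item's current static mesh to callers.
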(event `self.ReceiveBeginPlay`
  (`/Game/Blueprint/Interface/BI_Overlay.Overlay` false))

(event `/Game/Blueprint/Interface/BI_Overlay.Overlay`
  (params (True :type Boolean))
  (bind _widget (`self.Widget`))
  (bind _staticmeshcomponent (`self.StaticMeshComponent`))
  (if True
    (`MeshComponent.SetOverlayMaterial` _staticmeshcomponent "/Game/Material/MI_Outline.MI_Outline")
    (`SceneComponent.SetHiddenInGame` _widget false false)
    (else
      (`MeshComponent.SetOverlayMaterial` _staticmeshcomponent null)
      (`SceneComponent.SetHiddenInGame` _widget true false))))

(event `self.ReceiveAnyDamage`
  (params (Damage :type "Float (single-precision)") (DamageType :type "DamageType Object Reference") (InstigatedBy :type "Controller Object Reference") (DamageCauser :type "Actor Object Reference"))
  (`self.K2_DestroyActor`))

(fn `ReturnCurrentMesh`
  (returns (`Mesh ToReturn` :type "StaticMesh Object Reference"))
  (return (`StaticMeshComponent.StaticMesh` (`self.StaticMeshComponent`))))

(fn `UserConstructionScript`)