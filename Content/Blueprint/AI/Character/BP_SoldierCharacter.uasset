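; Soldier enemy character that carries a BP_Torch in each wrist socket and throws the left one when Shoot is called.
; BeginPlay spawns and attaches both torches and binds handlers for taking damage and seeing the player.
; Death flags the soldier dead, broadcasts EnemyDeath and notifies its controller; its animation and timed-cleanup code is disconnected.
; A stealth widget shows a timer percentage, hidden when updated after death.
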(event `self.ReceiveBeginPlay`
  (bind _returnvalue (`|SpawnActorFromClass` "/Game/Blueprint/AI/BP_Torch.BP_Torch_C" (`KismetMathLibrary.MakeTransform` (0.0 0.0 0.0)) "AlwaysSpawn" "MultiplyWithRoot" self self))
  (bind _output_get (set `self.TorchL` _returnvalue))
  (`self.K2_AttachToComponent` _output_get (`self.Mesh`) "Wrist_LSocket" "SnapToTarget" "SnapToTarget" "KeepRelative" false)
  (bind _returnvalue_2 (`|SpawnActorFromClass` "/Game/Blueprint/AI/BP_Torch.BP_Torch_C" (`KismetMathLibrary.MakeTransform` (0.0 0.0 0.0)) "AlwaysSpawn" "MultiplyWithRoot" self self))
  (bind _output_get_2 (set `self.TorchR` _returnvalue_2))
  (`self.K2_AttachToComponent` _output_get_2 (`self.Mesh`) "Wrist_RSocket" "SnapToTarget" "SnapToTarget" "KeepRelative" false)
  (add `self.OnTakeAnyDamage` (`|CreateDelegate` :!event `Death`))
  (add `self.OnEnemySeePlayer` (`|CreateDelegate` :!event `UpdateStealthIndicator`)))

(event `self.ReceivePossessed`
  (params (NewController :type "Controller Object Reference"))
  (set `self.New Controller` NewController))

(event `/Game/Blueprint/AI/Interface/BP_Shoot.Shoot`
  (params (Start :type "Vector Structure") (End :type "Vector Structure") (Velocity :type "Float (double-precision)"))
  (`/Game/Blueprint/AI/BP_Torch.Throw` (`self.TorchL`) Velocity Start End))

(fn `Death`
  (params (DamagedActor :type "Actor Object Reference") (Damage :type "Float (single-precision)") (DamageType :type "DamageType Object Reference") (InstigatedBy :type "Controller Object Reference") (DamageCauser :type "Actor Object Reference"))
  (locals (NewLocalVar :type "AnimationAsset Object Reference"))
  (bind _new_controller (`self.New Controller`))
  (`/Engine/EditorBlueprintResources/StandardMacros.IsValid` _new_controller
    (:`Is Valid`
      (`self.OnEnemyDeath` self)
      (set `self.bIsDied` true)
      (message `/Game/Blueprint/AI/Interface/BPI_Death.NotifyDeath` _new_controller))))

(fn `GetLeftWeapon`
  (returns (L_Weapon :type "/Game/Blueprint/AI/BP_Torch Object Reference"))
  (return (`self.TorchL`)))

(fn `GetRightWeapon`
  (returns (R_Weapon :type "/Game/Blueprint/AI/BP_Torch Object Reference"))
  (return (`self.TorchR`)))

(fn `UpdateStealthIndicator`
  (params (Percent :type "Float (single-precision)"))
  (if (`self.bIsDied`)
    (`SceneComponent.SetHiddenInGame` (`self.Widget`) true false)
    (else
      (`/Game/UI/WB_EnemyTimer.Set timer` (cast `/Game/UI/WB_EnemyTimer` (`WidgetComponent.GetWidget` (`self.Widget`)) :!pure true) Percent))))

(fn `UserConstructionScript`)