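; BP_Torch is a throwable torch for AI characters that damages non-AI actors it overlaps.
; Collision starts disabled; Throw enables it, detaches the torch and activates projectile and rotating movement.
; Launch velocity comes from SuggestProjectileVelocity as an arc between given start and end points, with debug drawing on.
; Capsule overlap applies damage credited to the owner, skipping the owner and GGJ_AIBaseCharacter actors.
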(event `self.ReceiveBeginPlay`
  (bind _returnvalue (`self.GetOwner`))
  (`self.DeactivateCollsion`)
  (`/Engine/EditorBlueprintResources/StandardMacros.IsValid` _returnvalue
    (:`Is Valid`
      (`PrimitiveComponent.IgnoreActorWhenMoving` (`self.Capsule`) _returnvalue true)
      (`PrimitiveComponent.IgnoreActorWhenMoving` (`self.Capsule`) self true))))

(event `Throw`
  (params (Velocity :type "Float (double-precision)") (Start :type "Vector Structure") (End :type "Vector Structure"))
  (bind _projectilemovement (`self.ProjectileMovement`))
  (set `ProjectileMovementComponent.MaxSpeed` Velocity _projectilemovement)
  (`self.ActivateCollsion`)
  (`self.K2_DetachFromActor` "KeepWorld" "KeepWorld" "KeepWorld")
  (`ActorComponent.Activate` (`self.ProjectileMovement`) false)
  (`ActorComponent.Activate` (`self.RotatingMovement`) false)
  (bind _tossvelocity (`GameplayStatics.BlueprintSuggestProjectileVelocity` Start End (`ProjectileMovementComponent.MaxSpeed` _projectilemovement) 0.0 "DoNotTrace" (`CapsuleComponent.GetScaledCapsuleRadius` (`self.Capsule`)) false true true))
  (set `MovementComponent.Velocity` _tossvelocity (`self.ProjectileMovement`)))

(event `self.Capsule.OnComponentBeginOverlap`
  (params (OverlappedComponent :type "PrimitiveComponent Object Reference") (OtherActor :type "Actor Object Reference") (OtherComp :type "PrimitiveComponent Object Reference") (OtherBodyIndex :type Integer) (bFromSweep :type Boolean) (SweepResult :type "HitResult Structure (by ref)"))
  (bind _returnvalue (`self.GetOwner`))
  (if (and (not (`KismetMathLibrary.ClassIsChildOf` (`GameplayStatics.GetObjectClass` OtherActor) "/Script/GGJ_Mask.GGJ_AIBaseCharacter")) (!= OtherActor _returnvalue))
    (`GameplayStatics.ApplyDamage` OtherActor 1.0 null _returnvalue)))

(fn `ActivateCollsion`
  (`PrimitiveComponent.SetCollisionEnabled` (`self.Capsule`) "QueryAndPhysics"))

(fn `DeactivateCollsion`
  (`PrimitiveComponent.SetCollisionEnabled` (`self.Capsule`) "NoCollision"))

(fn `UserConstructionScript`)