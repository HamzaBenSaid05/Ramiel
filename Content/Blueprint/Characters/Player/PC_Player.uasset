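; Player controller that sets up Enhanced Input and relays move and camera input to the controlled pawn through Move and Look messages.
; BeginPlay and Possess add the base mapping context, plus the advanced one if the pawn's class is exactly Character.
; UnPossess removes the base context, but checks for BP_Player before removing the advanced one.
; CreateHUD builds and displays the WB_Canvas widget, though nothing here calls it.
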(event `self.ReceiveBeginPlay`
  (`EnhancedInputSubsystemInterface.AddMappingContext` (subsystem `EnhancedInputLocalPlayerSubsystem`) "/Game/Blueprint/Characters/Player/IMC_PlayerBase.IMC_PlayerBase" 0 (struct))
  (if (== (`GameplayStatics.GetObjectClass` (`self.K2_GetPawn`)) "/Script/Engine.Character")
    (`EnhancedInputSubsystemInterface.AddMappingContext` (subsystem `EnhancedInputLocalPlayerSubsystem`) "/Game/Blueprint/Characters/Player/IMC_PlayerAdvanced.IMC_PlayerAdvanced" 0 (struct))))

(event `self.ReceivePossess`
  (params (PossessedPawn :type "Pawn Object Reference"))
  (`EnhancedInputSubsystemInterface.AddMappingContext` (subsystem `EnhancedInputLocalPlayerSubsystem`) "/Game/Blueprint/Characters/Player/IMC_PlayerBase.IMC_PlayerBase" 0 (struct))
  (if (== (`GameplayStatics.GetObjectClass` (`self.K2_GetPawn`)) "/Script/Engine.Character")
    (`EnhancedInputSubsystemInterface.AddMappingContext` (subsystem `EnhancedInputLocalPlayerSubsystem`) "/Game/Blueprint/Characters/Player/IMC_PlayerAdvanced.IMC_PlayerAdvanced" 0 (struct))))

(event `self.ReceiveUnPossess`
  (params (UnpossessedPawn :type "Pawn Object Reference"))
  (`EnhancedInputSubsystemInterface.RemoveMappingContext` (subsystem `EnhancedInputLocalPlayerSubsystem`) "/Game/Blueprint/Characters/Player/IMC_PlayerBase.IMC_PlayerBase" (struct))
  (if (== (`GameplayStatics.GetObjectClass` (`self.K2_GetPawn`)) "/Game/Blueprint/Characters/Player/BP_Player.BP_Player_C")
    (`EnhancedInputSubsystemInterface.RemoveMappingContext` (subsystem `EnhancedInputLocalPlayerSubsystem`) "/Game/Blueprint/Characters/Player/IMC_PlayerAdvanced.IMC_PlayerAdvanced" (struct))))

(event `EnhancedInput|/Game/Blueprint/Characters/Player/IA_Camera`
  (params (ActionValue :type "Vector2D Structure") (ElapsedSeconds :type "Float (double-precision)") (TriggeredSeconds :type "Float (double-precision)") (InputAction :type "InputAction Object Reference" :default "/Game/Blueprint/Characters/Player/IA_Camera.IA_Camera"))
  (:`Triggered`
    (message `/Game/Blueprint/Interface/BI_Possesable.Look` (`self.K2_GetPawn`) ActionValue_X ActionValue_Y)))

(event `EnhancedInput|/Game/Blueprint/Characters/Player/IA_Move`
  (params (ActionValue :type "Vector2D Structure") (ElapsedSeconds :type "Float (double-precision)") (TriggeredSeconds :type "Float (double-precision)") (InputAction :type "InputAction Object Reference" :default "/Game/Blueprint/Characters/Player/IA_Move.IA_Move"))
  (:`Triggered`
    (message `/Game/Blueprint/Interface/BI_Possesable.Move` (`self.K2_GetPawn`) ActionValue_X ActionValue_Y)))

(fn `Create HUD`
  (bind _returnvalue (`|CreateWidget` "/Game/UI/WB_Canvas.WB_Canvas_C" self))
  (bind _output_get (set `self.HUD` _returnvalue))
  (`UserWidget.AddToViewport` _output_get 0))

(fn `UserConstructionScript`)