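; Game mode for the mask game that tracks win conditions, updates the objective HUD and opens the king's door.
; On start it finds the door and all AI enemies, then binds death, key, priest-copy and door-attempt events.
; Killing every enemy, possessing the priest or a door-attempt event triggers the win, passing priest possession to the door's level sequence.
; Also records collected items and shows the game-over widget with UI-only input.
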(event `self.ReceiveBeginPlay`
  (`KismetSystemLibrary.DelayUntilNextTick`)
  (bind _returnvalue (`GameplayStatics.GetActorOfClass` "/Game/Blueprint/BP_KingDoor.BP_KingDoor_C"))
  (set `self.KingDoor` _returnvalue)
  (bind _outactors (`GameplayStatics.GetAllActorsOfClass` "/Script/GGJ_Mask.GGJ_AIBaseCharacter"))
  (bind _output_get (set `self.EnemyArray` _outactors))
  (for _array_element _output_get
    (add `GGJ_AIBaseCharacter.OnEnemyDeath` _array_element (`|CreateDelegate` :!event `EnemyDeath`)))
  (add `self.OnKeyCollected` (`|CreateDelegate` :!event `KeyCollected`))
  (add `self.OnPastorCopy` (`|CreateDelegate` :!event `PastorTransformation`))
  (add `self.OnTryOpenDoor` (delegate `TriggerWin`))
  (bind _asbp_player (cast `/Game/Blueprint/Characters/Player/BP_Player` (`GameplayStatics.GetPlayerPawn` 0)))
  (set `self.WB Objective` (`/Game/UI/WB_Canvas.WB_Objective` (`/Game/Blueprint/Characters/Player/BP_Player.HUD` _asbp_player))))

(event `TriggerWinKillAll`
  (`/Game/UI/WB_Objective.KilledEveryone` (`self.WB Objective`))
  (`self.TriggerWin`))

(event `TriggerWin`
  (bind _kingdoor (`self.KingDoor`))
  (`/Game/Blueprint/BP_KingDoor.OpenDoor` _kingdoor)
  (`/Game/Blueprint/BP_KingDoor.ChangeLevelSequence` _kingdoor (`self.bIsPriestPossesed`)))

(event `TriggerWhenPossessPriest`
  (`/Game/UI/WB_Objective.Find Relic and possessed priest` (`self.WB Objective`))
  (`self.TriggerWin`))

(fn `CollectItem`
  (params (ID :type Integer))
  (returns (True :type Boolean))
  (`KismetArrayLibrary.Array_AddUnique` (`self.CollectedItem`) ID)
  (`self.OnKeyCollected`)
  (return true))

(fn `EnemyDeath`
  (params (DestroyedActor :type "Actor Object Reference"))
  (bind _enemyarray (`self.EnemyArray`))
  (bind _asggj_aibase_character (cast `GGJ_AIBaseCharacter` DestroyedActor))
  (`KismetArrayLibrary.Array_RemoveItem` _enemyarray _asggj_aibase_character)
  (if (== (`KismetArrayLibrary.Array_Length` _enemyarray) 0)
    (`self.TriggerWinKillAll`)
    (`KismetSystemLibrary.PrintString` "Win")))

(fn `KeyCollected`
  (set `self.bHasKey` true)
  (`/Game/UI/WB_Objective.Find Relique` (`self.WB Objective`)))

(fn `PastorTransformation`
  (set `self.bIsPriestPossesed` true)
  (`self.TriggerWhenPossessPriest`))

(fn `SetGameOver`
  (params (IsWin :type Boolean))
  (bind _returnvalue (`GameplayStatics.GetPlayerController` 0))
  (bind _asbp_player (cast `/Game/Blueprint/Characters/Player/BP_Player` (`GameplayStatics.GetPlayerPawn` 0)))
  (`Widget.RemoveFromParent` (`/Game/Blueprint/Characters/Player/BP_Player.HUD` _asbp_player))
  (bind _returnvalue_2 (`|CreateWidget` "/Game/UI/WB_Gameover.WB_Gameover_C" (`GameplayStatics.GetPlayerController` 0)))
  (`UserWidget.AddToViewport` _returnvalue_2 0)
  (`/Game/UI/WB_Gameover.Set Gameover Text` _returnvalue_2 IsWin)
  (`WidgetBlueprintLibrary.SetInputMode_UIOnlyEx` _returnvalue _returnvalue_2)
  (set `PlayerController.bShowMouseCursor` true _returnvalue))

(fn `UserConstructionScript`)